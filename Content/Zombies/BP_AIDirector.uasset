(event `self.ReceiveTick`
  (params (DeltaSeconds :type "Float (single-precision)"))
  (bind _spawnrate (`self.SpawnRate`))
  (`|ExecutionSequence`
    (:`then_0`
      (if (`|EnumEquality` (`self.StateEnum`) "NewEnumerator3")
        (bind _result (`/Engine/EditorBlueprintResources/StandardMacros.DecrementFloat` (`self.RelaxTimer`))
          (:`  `
            (set `self.RelaxTimer` _result)
            (`KismetSystemLibrary.PrintString` (`|GetEnumeratorNameAsString` (`self.StateEnum`)) :!label _label)))))
    (:`then_1`
      (if (> _spawnrate 0.0)
        (bind _result_2 (`/Engine/EditorBlueprintResources/StandardMacros.DecrementFloat` _spawnrate)
          (:`  `
            (set `self.SpawnRate` _result_2)
            (goto _label)))))))

(event `self.ReceiveBeginPlay`
  (`self.DirectorState`)
  (`self.SpawningLogic`))

(event `/Game/Zombies/BPI_Director.GetStress`
  (params (Stress :type "Float (double-precision)"))
  (set `self.PlayerStress` Stress))

(event `/Game/Zombies/BPI_Director.DeadZombie`
  (`KismetArrayLibrary.Array_RemoveItem` (`self.ActiveZombies`)))

(event `DirectorState`
  (switch `/Game/Zombies/E_DirectorState` (`self.StateEnum`)
    (:`NewEnumerator0`
      (if (>= (`self.PlayerStress`) 55.0)
        (set `self.StateEnum` "NewEnumerator1")
        (set `self.SpawnRate` (`KismetMathLibrary.RandomFloatInRange` 3.0 5.0))
        (set `self.BatchAmount` (`KismetMathLibrary.RandomIntegerInRange` 5 15))
        (`self.DirectorState`)
        (else
          (`KismetSystemLibrary.K2_SetTimerDelegate` (delegate `DirectorState`) 1.5))))
    (:`NewEnumerator1`
      (if (>= (`self.PlayerStress`) 90.0)
        (set `self.StateEnum` "NewEnumerator2")
        (`self.DirectorState`)
        (else
          (`KismetSystemLibrary.K2_SetTimerDelegate` (delegate `DirectorState`) 1.5))))
    (:`NewEnumerator2`
      (if (< (`KismetArrayLibrary.Array_Length` (`self.ActiveZombies`)) 5)
        (set `self.StateEnum` "NewEnumerator3")
        (`self.DirectorState`)
        (else
          (`KismetSystemLibrary.K2_SetTimerDelegate` (delegate `DirectorState`) 1.5))))
    (:`NewEnumerator3`
      (if (<= (`self.RelaxTimer`) 0.0)
        (set `self.StateEnum` "NewEnumerator0")
        (set `self.RelaxTimer` 20.0)
        (set `self.SpawnRate` 40.0)
        (set `self.BatchAmount` 45)
        (`self.DirectorState`)
        (else
          (`KismetSystemLibrary.K2_SetTimerDelegate` (delegate `DirectorState`) 1.5))))))

(event `SpawningLogic`
  (switch `/Game/Zombies/E_DirectorState` (`self.StateEnum`)
    (:`NewEnumerator0`
      (if (and (<= (`self.SpawnRate`) 0.0) (!= (`KismetArrayLibrary.Array_Length` (`self.ActiveZombies`)) (`self.Limit`)))
        (for _ (range (+ (`self.BatchAmount`) 1))
          (bind _randomlocation (`NavigationSystemV1.K2_GetRandomLocationInNavigableRadius` (2400.0 1360.0 75.0) 2000.0 null "/Script/AIModule.NavFilter_AIControllerDefault"))
          (bind _returnvalue (`|SpawnActorFromClass` "/Game/Zombies/ZombieFemale/Meshes-textures/BP_ZombieFemale.BP_ZombieFemale_C" (`KismetMathLibrary.Conv_VectorToTransform` _randomlocation) "Undefined" "MultiplyWithRoot" null null))
          (`KismetArrayLibrary.Array_AddUnique` (`self.ActiveZombies`) _returnvalue)
          (if (`|EnumEquality` (`self.StateEnum`) "NewEnumerator1")
            (break)))
        (set `self.SpawnRate` 40.0)
        (set `self.BatchAmount` 45)
        (`self.SpawningLogic`)
        (else
          (`KismetSystemLibrary.K2_SetTimerDelegate` (delegate `SpawningLogic`) 1.0))))
    (:`NewEnumerator1`
      (if (and (<= (`self.SpawnRate`) 0.0) (!= (`KismetArrayLibrary.Array_Length` (`self.ActiveZombies`)) (`self.Limit`)))
        (for _ (range (+ (`self.BatchAmount`) 1))
          (bind _randomlocation_2 (`NavigationSystemV1.K2_GetRandomLocationInNavigableRadius` (2400.0 1360.0 75.0) 2000.0 null "/Script/AIModule.NavFilter_AIControllerDefault"))
          (bind _returnvalue_2 (`|SpawnActorFromClass` "/Game/Zombies/ZombieFemale/Meshes-textures/BP_ZombieFemale.BP_ZombieFemale_C" (`KismetMathLibrary.Conv_VectorToTransform` _randomlocation_2) "Undefined" "MultiplyWithRoot" null null))
          (`KismetArrayLibrary.Array_AddUnique` (`self.ActiveZombies`) _returnvalue_2)
          (if (`|EnumEquality` (`self.StateEnum`) "NewEnumerator2")
            (break)))
        (set `self.SpawnRate` (`KismetMathLibrary.RandomFloatInRange` 3.0 5.0))
        (set `self.BatchAmount` (`KismetMathLibrary.RandomIntegerInRange` 5 15))
        (`self.SpawningLogic`)
        (else
          (`KismetSystemLibrary.K2_SetTimerDelegate` (delegate `SpawningLogic`) 1.0))))
    (:`NewEnumerator2`
      (`self.SpawningLogic`))
    (:`NewEnumerator3`
      (`self.SpawningLogic`))))

(fn `UserConstructionScript`)