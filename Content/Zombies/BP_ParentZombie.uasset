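; Base zombie class that handles damage, hit reactions and death, with stub functions such as HitAnim and StressVal presumably left for child Blueprints.
; Non-lethal hits play a montage; death notifies the GameMode, disables capsule collision and movement, and launches the mesh as a ragdoll.
; A timeline then drives a shared alpha on a dynamic disintegration material and Niagara effect before the actor is destroyed, which notifies the GameMode again.
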(event `self.ReceiveDestroyed`
  (message `/Game/Zombies/BPI_Director.DeadZombie` (`GameplayStatics.GetGameMode`)))

(event `/Game/FirstPerson/Blueprints/BPI_Combat.TakeDamage`
  (params (Damage :type "Float (double-precision)") (HitSpot :type "Vector Structure"))
  ; DamageLogic
  (bind _output_get (set `self.Health` (- (`self.Health`) Damage)))
  (`/Game/FirstPerson/Blueprints/BPI_Combat.IsDead?` _output_get))

(event `/Game/FirstPerson/Blueprints/BPI_Combat.IsDead?`
  (params (Health :type "Float (double-precision)"))
  (bind _mesh (`self.Mesh`))
  ; DamageLogic
  (if (<= Health 0.0)
    (set `self.Dead?` true)
    (`/Engine/EditorBlueprintResources/StandardMacros.DoOnce` false
      (:`Completed`
        (`PrimitiveComponent.SetSimulatePhysics` _mesh true)
        (`PrimitiveComponent.SetCollisionProfileName` (`self.CapsuleComponent`) "NoCollision" false)
        (`self.EffecientDeath`)
        (message `/Game/Zombies/BPI_Director.DeadZombie` (`GameplayStatics.GetGameMode`))
        (`PrimitiveComponent.AddImpulse` (`self.Mesh`) (* (stale `/Game/FirstPerson/Blueprints/BPI_Combat.TakeDamage` HitSpot) 1500.0) "None" false)
        (`self.Disintegrate` "NewEnumerator0")
        (`GameplayStatics.SpawnSoundAttached` "/Game/FirstPerson/SFX/MetaSounds/MSS_Disintegrate.MSS_Disintegrate" (`self.Mesh`) "None" (0.0 0.0 0.0) (struct) "KeepRelativeOffset" false 0.5 1.0 0.0 "/Game/FirstPerson/SFX/Attenuation/Disintegrate_Attenuation.Disintegrate_Attenuation" null)
        (`self.IsDead`)))
    (else
      (bind _deathanim (`/Game/Zombies/BPI_Zombie.HitAnim`))
      (`|PlayMontage` _mesh _deathanim
        (:`then`
          (set `self.bHit` true))
        (:`OnCompleted`
          (set `self.bHit` false))))))

(event `EffecientDeath`
  (`SkeletalMeshComponent.SetAnimation` (`self.Mesh`) null)
  (`ActorComponent.Deactivate` (`self.CharacterMovement`)))

(event `Disintegrate`
  (params (WeaponType :type "/Game/FirstPerson/Weapons/Enum_WeaponType Enum" :default "NewEnumerator0"))
  (`KismetSystemLibrary.Delay` 0.25)
  (`self.DeathMaterialCyber`)
  (`ActorComponent.Activate` (`self.Niagara`) false)
  (bind (_direction _newtrack_0) (`Timeline|Timeline` :!via `PlayFromStart`)
    (:`Update`
      (`MaterialInstanceDynamic.SetScalarParameterValue` (`self.DynamicMaterial`) "Alpha" _newtrack_0)
      (`NiagaraComponent.SetVariableFloat` (`self.Niagara`) "Alpha" _newtrack_0))
    (:`Finished`
      (`ActorComponent.Deactivate` (`self.Niagara`))
      (`KismetSystemLibrary.K2_SetTimerDelegate` (delegate `Dead`) 0.9))))

(event `Dead`
  (`self.K2_DestroyActor`))

(event `DeathMaterialCyber`
  (if (`KismetSystemLibrary.IsValid` (`self.DeathMesh`))
    (bind _returnvalue (`PrimitiveComponent.CreateDynamicMaterialInstance` (`self.DeathMesh`) 0 "/Game/FirstPerson/Weapons/M_Disintagrate.M_Disintagrate" "None"))
    (set `self.DynamicMaterial` _returnvalue)
    (`NiagaraComponent.SetAsset` (`self.Niagara`) "/Game/FirstPerson/Weapons/NS_Disintagrate.NS_Disintagrate" true)
    (for _index (range 3)
      (`PrimitiveComponent.SetMaterial` (`self.DeathMesh`) _index (`self.DynamicMaterial`))
      (`MaterialInstanceDynamic.SetScalarParameterValue` (`self.DynamicMaterial`) "Alpha" 0.0))))

(fn `AddCharge`
  (params (ChargeValue :type Integer))
  (returns (Charge :type "Float (double-precision)"))
  (if (`self.Dead?`)
    (return (select `int` ChargeValue :`0` 0.0 :`1` 1.0 :`2` 2.5 :`3` 5.0 :`4` 10.0))))

(fn `ArrayCheck`
  (params (HoldInt :type Integer))
  (returns (OutputInt :type Integer))
  (bind _returnvalue (`KismetArrayLibrary.Array_LastIndex` (`self.StateArray`)))
  (if (> HoldInt _returnvalue)
    (return _returnvalue)
    (else
      (return HoldInt))))

(fn `DeadCheck`
  (returns (Dead :type Boolean))
  (return false))

(fn `HitAnim`
  (returns (DeathAnim :type "AnimMontage Object Reference"))
  (return null))

(fn `StressVal`
  (returns (Stress :type "Float (double-precision)"))
  (return 0.0))

(fn `UserConstructionScript`)