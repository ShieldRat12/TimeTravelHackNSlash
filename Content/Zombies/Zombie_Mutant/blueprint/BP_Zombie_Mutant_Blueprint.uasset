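; Mutant zombie enemy Blueprint that speeds up on seeing the first-person player, chases and melee attacks.
; RunPlayer uses AIMoveTo toward the player controller, leading to AttackPlayer on success.
; The attack montage's notify triggers delayed sphere overlaps at an arrow, damaging the player and nearby zombies.
; RunToPlayer, called to resume the chase, is empty here, and the breathing morph-target timeline is unconnected.
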(event `self.ReceiveBeginPlay`)

(event `self.PawnSensing.OnSeePawn`
  (params (Pawn :type "Pawn Object Reference"))
  (if (== Pawn "/Game/FirstPerson/Blueprints/BP_FirstPersonCharacter.BP_FirstPersonCharacter")
    (set `self.See Player` true)
    (set `CharacterMovementComponent.MaxWalkSpeed` 360.0 (`self.CharacterMovement`))))

(event `RunPlayer`
  (if (not (`self.Dead?_0`))
    (`|AIMoveTo` self (0.0 0.0 0.0) (`GameplayStatics.GetPlayerController` 0) 90.0 true
      (:`OnSuccess`
        (`self.AttackPlayer`))
      (:`OnFail`
        (`self.RunToPlayer`)))))

(event `AttackPlayer`
  (bind _array (`|MakeArray` "ObjectTypeQuery3" :!type "EObjectTypeQuery Enum"))
  (bind _returnvalue (`SceneComponent.K2_GetComponentLocation` (`self.Arrow1`)))
  (bind _array_2 (`|MakeArray` self :!type "Actor Object Reference"))
  (if (not (`self.bHit`))
    (`|PlayMontage` (`self.Mesh`) "/Game/Zombies/ZombieFemale/Anims/zombie_attack_Montage2.zombie_attack_Montage2"
      (:`OnCompleted`
        (`self.RunToPlayer` :!label _label))
      (:`OnInterrupted`
        (goto _label))
      (:`OnNotifyBegin`
        (`KismetSystemLibrary.Delay` 0.325)
        (bind (_outactors _returnvalue_2) (`KismetSystemLibrary.SphereOverlapActors` _returnvalue 100.0 _array "/Game/FirstPerson/Blueprints/BP_FirstPersonCharacter.BP_FirstPersonCharacter_C" _array_2))
        (for _array_element _outactors
          (if (and _returnvalue_2 (`KismetSystemLibrary.IsValid` _array_element))
            (message `/Game/FirstPerson/Blueprints/BPI_Combat.TakeDamage` _array_element 5.0 (0.0 0.0 0.0))))
        (bind (_outactors_2 _returnvalue_3) (`KismetSystemLibrary.SphereOverlapActors` _returnvalue 40.0 _array "/Game/Zombies/BP_ParentZombie.BP_ParentZombie_C" _array_2))
        (for _array_element_2 _outactors_2
          (if (and _returnvalue_3 (`KismetSystemLibrary.IsValid` _array_element_2))
            (message `/Game/FirstPerson/Blueprints/BPI_Combat.TakeDamage` _array_element_2 5.0 (0.0 0.0 0.0))))))
    (else
      (`self.RunToPlayer`))))

(fn `RunToPlayer`)

(fn `UserConstructionScript`)